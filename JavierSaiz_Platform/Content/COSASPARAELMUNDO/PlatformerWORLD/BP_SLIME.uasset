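; BP_SLIME is a platformer slime enemy that patrols and damages the player on overlap.
; On BeginPlay a timeline animates the Slime component's Y and Z scale while GuardPatrol starts a slow AIMoveTo through the PatrolLocation array.
; Each successful move waits randomly, re-calls GuardPatrol, then increments the index, wrapping at four.
; Overlapping BP_Character_Chica applies fixed damage; an older FlipFlop movement attempt is left unconnected.
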(event Custom|GuardPatrol
  ;[1 1 1] Movimiento Slime
  (Variables|/Script/Engine.CharacterMovementComponent|SetMaxWalkSpeed (Variables|Character|GetCharacterMovement) 1.5e+02)
  (AI|AIMoveTo self (Utilities|Array|Get(acopy) (Variables|Default|GetPatrolLocation) (Variables|Default|GetLocations)) 0 5.0 false
    (:OnSuccess
      (Utilities|FlowControl|Delay (Math|Random|RandomFloatinRange 0.5 2.0))
      (CallFunction|GuardPatrol)
      (Math|Integer|IncrementInt (Variables|Default|GetLocations)
        (:%20%20
          (if (== (Variables|Default|GetLocations) 4)
            (Variables|Default|SetLocations 0)))))))

(event EventBeginPlay
  (CallFunction|GuardPatrol)
  (bind (_direction _scaley _scalez) (Timeline|Timeline Play)
    (:Update
      (Transformation|SetRelativeScale3D (Variables|Default|Getslime) (Math|Vector|MakeVector 1.0 _scaley _scalez)))))

(event Collision|EventActorBeginOverlap
  (params (OtherActor :type Actor%20Object%20Reference))
  ;[1 1 1] Daño a jugador
  (bind _asbp_character_chica (Utilities|Casting|CastToBP_Character_Chica OtherActor))
  (Game|Damage|ApplyDamage _asbp_character_chica 25.0 0 0 "/Script/Engine.DamageType")
  (Utilities|FlowControl|Delay 0.5))

(event EventTick
  (params (DeltaSeconds :type Float%20%28single-precision%29))
  ;[1 1 1] Movimiento Slime
)

(fn ConstructionScript)